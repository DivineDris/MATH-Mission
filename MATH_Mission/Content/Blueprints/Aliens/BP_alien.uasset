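; BP_alien is the alien actor the player must catch; overlapping it triggers the win message on the player and the BPW_UI widget.
; Each tick it moves along X by an accumulated speed offset from its start transform, copying the player's Y and keeping its initial Z.
; IncreaseSpeed, on a hit, briefly reverses and offsets the speed, restores it after a delay, then later calls SetFalseMessage on the player.
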(event `self.ReceiveBeginPlay`
  (`self.Initialize`))

(event `self.ReceiveTick`
  (params (DeltaSeconds :type "Float (single-precision)"))
  (`self.Movement`))

(event `/Game/Blueprints/Aliens/BPI_SpeedUp.IncreaseSpeed`
  (params (IsHited :type Boolean))
  (if IsHited
    (set `self.MovementSpeed` (* (+ (`self.MovementSpeed`) (`self.SpeedScale`)) -1.0))
    (`KismetSystemLibrary.Delay` 0.7)
    (set `self.MovementSpeed` (* (+ (`self.MovementSpeed`) (`self.SpeedScale`)) -1.0))
    (`KismetSystemLibrary.Delay` 1.0)
    (message `/Game/Blueprints/Player/BPI_SetIsHitedFalse.SetFalse` (`GameplayStatics.GetPlayerPawn` 0))))

(event `self.ReceiveActorBeginOverlap`
  (params (OtherActor :type "Actor Object Reference"))
  (if (== OtherActor (`GameplayStatics.GetPlayerPawn` 0))
    (bind _foundwidgets (`WidgetBlueprintLibrary.GetAllWidgetsOfClass` "/Game/Blueprints/HUD/BPW_UI.BPW_UI_C"))
    (message `/Game/Blueprints/HUD/BPI_VictoryScreen.WinTheGame` (`|GetArrayItem` _foundwidgets))
    (message `/Game/Blueprints/HUD/BPI_VictoryScreen.WinTheGame` (`GameplayStatics.GetPlayerPawn` 0))))

(fn `Initialize`
  (set `self.AlienTransform` (`self.GetTransform` self)))

(fn `Movement`
  (bind _alientransform (`self.AlienTransform`))
  (bind (_returnvalue_x _returnvalue_y) (`KismetMathLibrary.BreakVector` (`self.K2_GetActorLocation` (`GameplayStatics.GetPlayerPawn` 0))))
  (bind _output_get (set `self.MovementDistance` (+ (`self.MovementDistance`) (* (`self.MovementSpeed`) -1.0))))
  (`self.K2_SetActorLocation` (`KismetMathLibrary.MakeVector` (+ _output_get (.x (.location _alientransform))) _returnvalue_y (.z (.location _alientransform)))))

(fn `UserConstructionScript`)
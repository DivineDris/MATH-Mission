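; BP_Rocket_1 is the player-controlled rocket, which slides sideways along Y within fixed bounds through the Enhanced Input move action.
; On BeginPlay it adds the input mapping, caches the first BP_alien in the level and starts a looping 2D sound.
; HitObstacle tells the alien to increase speed, guarded by a hit flag that SetFalse clears.
; TimerStoped and WintheGame both stop the sound.
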(event `self.ReceiveBeginPlay`
  (bind _asplayer_controller (cast `PlayerController` (`self.GetController`)))
  (bind _returnvalue (pcsubsystem `EnhancedInputLocalPlayerSubsystem` _asplayer_controller))
  (`/Engine/EditorBlueprintResources/StandardMacros.IsValid` _returnvalue
    (:`Is Valid`
      (`EnhancedInputSubsystemInterface.AddMappingContext` _returnvalue "/Game/ThirdPerson/Input/IMC_Default.IMC_Default" 0 (struct))
      (`self.Initialize`)
      (bind _returnvalue_2 (`GameplayStatics.SpawnSound2D` "/Game/Sound/217603__zagi2__magnetic-loop.217603__zagi2__magnetic-loop" 1.0 1.0 0.0 null))
      (set `self.Audio` _returnvalue_2))))

(event `EnhancedInput|/Game/ThirdPerson/Input/Actions/IA_Move`
  (params (ActionValue :type "Vector2D Structure") (ElapsedSeconds :type "Float (double-precision)") (TriggeredSeconds :type "Float (double-precision)") (InputAction :type "InputAction Object Reference" :default "/Game/ThirdPerson/Input/Actions/IA_Move.IA_Move"))
  (:`Triggered`
    (`self.Rocket Control` ActionValue_X)))

(event `/Game/Blueprints/Player/BPI_HitObstacle.HitObstacle`
  (if (not (`self.IsHited`))
    (set `self.IsHited` true)
    (`/Game/Blueprints/Aliens/BP_alien.IncreaseSpeed` (`self.Alien`) (`self.IsHited`))))

(event `/Game/Blueprints/Player/BPI_SetIsHitedFalse.SetFalse`
  (set `self.IsHited` false))

(event `/Game/Blueprints/Player/BPI_Timer.TimerStoped`
  (`AudioComponent.Stop` (`self.Audio`)))

(event `/Game/Blueprints/HUD/BPI_VictoryScreen.WinTheGame`
  (`AudioComponent.Stop` (`self.Audio`)))

(fn `Initialize`
  (bind _outactors (`GameplayStatics.GetAllActorsOfClass` "/Game/Blueprints/Aliens/BP_alien.BP_alien_C"))
  (set `self.Alien` (`|GetArrayItem` _outactors)))

(fn `Rocket Control`
  (params (float :type "Float (double-precision)"))
  (bind (_returnvalue_x _returnvalue_y _returnvalue_z) (`KismetMathLibrary.BreakVector` (`self.K2_GetActorLocation`)))
  (bind _returnvalue (+ _returnvalue_y (* float (`self.MovementDistance`))))
  (if (and (< _returnvalue 210.0) (> _returnvalue -210.0))
    (`self.K2_SetActorLocation` (`KismetMathLibrary.MakeVector` _returnvalue_x _returnvalue _returnvalue_z))))

(fn `UserConstructionScript`)
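; BP_BaseObstacle is a base obstacle actor that slides along negative world X and reacts when it hits the player.
; On BeginPlay it caches its starting transform, then each Tick adds an accumulated offset to that start location.
; MovementSpeed is applied per frame without delta time, so movement depends on frame rate.
; Overlapping the first player's pawn sends it HitObstacleMessage, then destroys the obstacle.
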(event `self.ReceiveBeginPlay`
  (`self.Initialise`))

(event `self.ReceiveActorBeginOverlap`
  (params (OtherActor :type "Actor Object Reference"))
  (bind _returnvalue (`GameplayStatics.GetPlayerPawn` 0))
  (if (== OtherActor _returnvalue)
    (message `/Game/Blueprints/Player/BPI_HitObstacle.HitObstacle` _returnvalue)
    (`self.K2_DestroyActor`)))

(event `self.ReceiveTick`
  (params (DeltaSeconds :type "Float (single-precision)"))
  (bind _transform (`self.Transform`))
  (bind _output_get (set `self.MovementDistance` (+ (`self.MovementDistance`) (* (`self.MovementSpeed`) -1.0))))
  (`self.K2_SetActorTransform` (`self.ThisActor`) (`KismetMathLibrary.MakeTransform` (`KismetMathLibrary.MakeVector` (+ _output_get (.x (.location _transform))) (.y (.location _transform)) (.z (.location _transform)))) false false))

(fn `Initialise`
  (bind _output_get (set `self.ThisActor` self))
  (set `self.Transform` (`self.GetTransform` _output_get)))

(fn `UserConstructionScript`)